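; GM_FIH is the game mode that drives a step-based fish-catching progression and creates the HUD, fade-to-black and new-upgrade widgets.
; Each step fills a map of fish to catch, broadcasts list updates, and makes fish splines of matching classes spawn their fish.
; Grabbing marks a fish caught; redeeming a complete list plays the upgrade animation and advances to the next step.
; It also exposes the death fade animation.
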(event Custom|FadeBlackDie
  (Default|PlayFadeBlackAnim (Variables|Default|GetFadeBlack%20HUD)))

(event Custom|SpawnFishOnSplines
  (bind _keypin (Utilities|Map|ForEachLoop(Map) (Variables|Default|GetFishToCatch))
    (:then
      (Utilities|Array|Add (Variables|Default|GetCurrentClasses) (Variables|/Game/01-Blueprints/GPE/Fishes/BP_DA_Fish.BP_DA_Fish_C|GetFishClass _keypin)))
    (:CompletedPin
      (bind _outactors (Actor|GetAllActorsOfClass "/Game/01-Blueprints/GPE/BP_FishSpline.BP_FishSpline_C"))
      (for _array_element _outactors
        (if (Utilities|Array|ContainsItem (Variables|Default|GetCurrentClasses) (Variables|/Game/01-Blueprints/GPE/BP_FishSpline.BP_FishSpline_C|GetFishClass _array_element))
          (Default|SpawnFishes _array_element))))))

(event Custom|RedeemFish
  (if (CallFunction|HasAllFishes)
    (Utilities|Map|Clear (Variables|Default|GetFishToCatch))
    (Default|LaunchAnim (Variables|Default|GetNewUpgrade) (.MemberVar_6 (Utilities|Struct|BreakSFishStep (Utilities|Array|Get(acopy) (Variables|Default|GetSteps) (Variables|Default|GetCurrentStep)))))
    (Math|Integer|IncrementInt (Variables|Default|GetCurrentStep)
      (:%20%20
        (CallFunction|UpdateListtoCatch)
        (CallFunction|SpawnFishonSplines)))))

(event EventBeginPlay
  (Input|SetInputModeGameOnly (Game|GetPlayerController 0) false)
  (bind _returnvalue (UserInterface|CreateWidget "/Game/01-Blueprints/Uis/WBP_Hud.WBP_Hud_C"))
  (bind _output_get (Variables|Default|SetHUD%20Chara _returnvalue))
  (UserInterface|Viewport|AddtoViewport _output_get 0)
  (bind _returnvalue_2 (UserInterface|CreateWidget "/Game/01-Blueprints/Uis/WBP_FadeBlack.WBP_FadeBlack_C"))
  (bind _output_get_2 (Variables|Default|SetFadeBlack%20HUD _returnvalue_2))
  (UserInterface|Viewport|AddtoViewport _output_get_2 5)
  (bind _returnvalue_3 (UserInterface|CreateWidget "/Game/01-Blueprints/Uis/WBP_NewUpgrade.WBP_NewUpgrade_C"))
  (bind _output_get_3 (Variables|Default|SetNewUpgrade _returnvalue_3))
  (UserInterface|Viewport|AddtoViewport _output_get_3 10)
  (CallFunction|UpdateListtoCatch)
  (CallFunction|SpawnFishonSplines))

(fn ConstructionScript)

(fn SetGrabFish
  (params (Fish%20DA :type BP%20DA%20Fish%20Object%20Reference))
  (bind _fishtocatch (Variables|Default|GetFishToCatch))
  (Utilities|Map|Add _fishtocatch Fish%20DA true)
  (Default|CallOnListUpdate _fishtocatch))

(fn HasAllFishes
  (bind _valuepin (Utilities|Map|ForEachLoop(Map) (Variables|Default|GetFishToCatch) :!label _label)
    (:then
      (if (not _valuepin)
        (LocalVariables|SetFound true)
        (goto _label BreakPin)))
    (:CompletedPin
      (return (not (LocalVariables|GetFound))))))

(fn UpdateListtoCatch
  (for _array_element (.Fishes (Utilities|Struct|BreakSFishStep (Utilities|Array|Get(acopy) (Variables|Default|GetSteps) (Variables|Default|GetCurrentStep))))
    (Utilities|Map|Add (Variables|Default|GetFishToCatch) _array_element false))
  (Default|CallOnListUpdate (Variables|Default|GetFishToCatch)))