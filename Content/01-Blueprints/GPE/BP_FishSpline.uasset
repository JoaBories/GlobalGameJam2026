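; BP_FishSpline spawns a school of fish actors that swim in a loop along a spline.
; Each fish gets a random start distance and a random offset, and a map stores its distance along the spline.
; A looping timer, used instead of Tick, advances each fish by its speed, restarts it at the spline's start and drops invalid ones.
; A sine wave along the up vector adds undulation, and look-ahead sampling sets facing.
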(event Custom|SpawnFish
  (bind _returnvalue (Math|Random|RandomFloat))
  (bind _fishes (Variables|Default|GetFishes))
  (bind _returnvalue_2 (Game|SpawnActorfromClass (Variables|Default|GetFishClass) (Math|Transform|MakeTransform "0, 0, 0" "0, 0, 0" "1.000000,1.000000,1.000000") "AdjustIfPossibleButAlwaysSpawn" "MultiplyWithRoot" 0 0))
  (Utilities|Map|Add _fishes _returnvalue_2 (Math|Random|RandomFloatinRange 0.0 (Spline|GetSplineLength (Variables|Default|GetSpline))))
  (bind _output_get (Variables|/Game/01-Blueprints/GPE/Fishes/BP_FishBase.BP_FishBase_C|SetOffset _returnvalue_2 (* (+ (* (Class|KismetMathLibrary|VectorRight) _returnvalue) (* (Math|Vector|VectorUp) _returnvalue) (* (Class|KismetMathLibrary|VectorForward) _returnvalue)) (Variables|Default|GetOffsetSize))))
  (Transformation|SetActorLocationAndRotation _returnvalue_2 (+ (.Pos (CallFunction|GetPosRotAlongSpline (.Value (Utilities|Map|Find _fishes _returnvalue_2)))) _output_get) (.Rot (CallFunction|GetPosRotAlongSpline (.Value (Utilities|Map|Find _fishes _returnvalue_2))))))

(event Custom|SpawnFishes
  (if (Utilities|Map|IsEmpty (Variables|Default|GetFishes))
    (for _index (range 0 (- (Variables|Default|GetFishNumber) 1))
      (CallFunction|SpawnFish))
    (CallFunction|StartFishesTick)
    (Variables|Default|Setchara_ref (Game|Player|GetPlayerPawn 0))))

(event Custom|start%20fishes%20tick
  (Utilities|Time|SetTimerbyEvent (delegate Custom|fish%20tick) 0.05 true true))

(event Custom|fish%20tick
  (bind _output_get (Variables|Default|Setdelta%20time 0.05))
  (if (Utilities|Map|IsNotEmpty (Variables|Default|GetFishes))
    (bind (_keypin _valuepin) (Utilities|Map|ForEachLoop(Map) (Variables|Default|GetFishes))
      (:then
        (Utilities|IsValid _keypin
          (:Is%20Valid
            (CallFunction|UpdateFish _keypin _valuepin _output_get))
          (:Is%20Not%20Valid
            (Utilities|Map|Remove (Variables|Default|GetFishes) _keypin)))))))

(event EventBeginPlay
  (if (Variables|Default|GetAutoSpawn)
    (CallFunction|SpawnFishes)))

(event EventTick
  (params (DeltaSeconds :type Float%20%28single-precision%29)))

(fn ConstructionScript)

(fn GetPosAlongSpline
  (params (CoordOnSpline :type Float%20%28double-precision%29))
  (bind _spline (Variables|Default|GetSpline))
  (return (+ (* (* (Math|Trig|Sin(Degrees) (* (Variables|Default|GetOscillationFrequency) CoordOnSpline)) (Variables|Default|GetOscillationAmplitude)) (Class|SplineComponent|GetUpVectoratDistanceAlongSpline _spline CoordOnSpline "World")) (Spline|GetLocationatDistanceAlongSpline _spline CoordOnSpline "World"))))

(fn UpdateFish
  (params (Fish :type BP%20Fish%20Base%20Object%20Reference) (CurrentPos :type Float%20%28double-precision%29) (DeltaTime :type Float%20%28double-precision%29))
  (bind _fishspeed (Variables|/Game/01-Blueprints/GPE/Fishes/BP_FishBase.BP_FishBase_C|GetFishSpeed Fish))
  (bind _spline (Variables|Default|GetSpline))
  (bind _returnvalue (Spline|GetSplineLength _spline))
  (bind _returnvalue_2 (* _fishspeed DeltaTime))
  (bind _returnvalue_3 (+ CurrentPos _returnvalue_2))
  (bind _returnvalue_4 (>= _returnvalue_3 _returnvalue))
  (bind _returnvalue_5 (Math|Float|SelectFloat 0.0 _returnvalue_3 _returnvalue_4))
  (bind (_pos _rot) (CallFunction|GetPosRotAlongSpline _returnvalue_5))
  (Transformation|SetActorLocationAndRotation Fish (+ (Variables|/Game/01-Blueprints/GPE/Fishes/BP_FishBase.BP_FishBase_C|GetOffset Fish) _pos) _rot)
  (Utilities|Map|Add (Variables|Default|GetFishes) Fish _returnvalue_5))

(fn GetPosRotAlongSpline
  (params (CoordOnSpline :type Float%20%28double-precision%29))
  (bind _output_get (LocalVariables|SetCurrentPos (CallFunction|GetPosAlongSpline CoordOnSpline)))
  (return _output_get (Math|Rotator|FindLookatRotation (LocalVariables|GetCurrentPos) (CallFunction|GetPosAlongSpline (+ CoordOnSpline 1.0)))))