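; BP_Shop is a shop actor that runs scripted dialogues with the diver player.
; LaunchDialogue puts the diver in dialogue mode and uses a timeline to glide them to a scene point while turning their view toward the SMLaurent mesh.
; NextLine then steps through the current dialogue's lines in a WBP_Dialogue widget, hiding it and advancing to the next dialogue at the end.
; It also binds to the game mode's list update, but that handler is empty.
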(event Custom|UpdateList
  (params (List :type Map%20of%20BP%20DA%20Fish%20Object%20References%20to%20Booleans)))

(event Custom|LaunchDialogue
  (bind _bpdiver (Variables|Default|GetBPDiver))
  (Default|GoinDialogue (Variables|Default|GetBPDiver))
  (Variables|Default|SetStartLocation (Transformation|GetActorLocation _bpdiver))
  (Variables|Default|SetStartRotation (Pawn|GetControlRotation _bpdiver :!class /Script/Engine.Pawn))
  (bind _newtrack_0 (Timeline|MovePlayer PlayFromStart)
    (:Update
      (Transformation|SetActorLocation (Variables|Default|GetBPDiver) (Math|Vector|Lerp(Vector) (Variables|Default|GetStartLocation) (Transformation|GetWorldLocation (Variables|Default|GetScene)) _newtrack_0) false false)
      (Pawn|SetControlRotation (Game|GetPlayerController 0) (Math|Rotator|Lerp(Rotator) (Variables|Default|GetStartRotation) (Variables|Default|GetLookAtRotation) _newtrack_0 true)))
    (:Finished
      (Widget|SetRenderOpacity (Variables|Default|GetDialogueWidget) 1.0)
      (CallFunction|NextLine))))

(event Custom|NextLine
  (bind _dialogues (Variables|Default|GetDialogues))
  (bind _currentdialogue (Variables|Default|GetcurrentDialogue))
  (bind _output (Utilities|Array|Get(acopy) _dialogues _currentdialogue))
  (bind _result (Math|Integer|IncrementInt (Variables|Default|GetcurrentLine))
    (:%20%20
      (if (>= _result (Utilities|Array|Length (.dialogues _output)))
        (Default|ExitDialogue (Variables|Default|GetBPDiver))
        (Widget|SetRenderOpacity (Variables|Default|GetDialogueWidget) 0.0)
        (Variables|Default|SetcurrentLine -1)
        (Math|Integer|IncrementInt (Variables|Default|GetcurrentDialogue))
        (else
          (Default|SetText (Variables|Default|GetDialogueWidget) (Utilities|Array|Get(acopy) (.dialogues _output) (Variables|Default|GetcurrentLine))))))))

(event EventBeginPlay
  (bind _asgm_fih (Utilities|Casting|CastToGM_FIH (Game|GetGameMode)))
  (bind _output_get (Variables|Default|SetGamemode _asgm_fih))
  (EventDispatchers|BindEventtoOnListUpdate _output_get (delegate Custom|UpdateList))
  (bind _asbp_diver (Utilities|Casting|CastToBP_Diver (Game|Player|GetPlayerPawn 0)))
  (Variables|Default|SetBPDiver _asbp_diver)
  (bind _returnvalue (Game|ConstructObjectfromClass "/Game/01-Blueprints/Uis/WBP_Dialogue.WBP_Dialogue_C"))
  (bind _output_get_2 (Variables|Default|SetDialogueWidget _returnvalue))
  (UserInterface|Viewport|AddtoViewport _output_get_2 15)
  (Widget|SetRenderOpacity _output_get_2 0.0)
  (Variables|Default|SetLookAtRotation (Math|Rotator|FindLookatRotation (Transformation|GetWorldLocation (Variables|Default|GetScene)) (Transformation|GetWorldLocation (Variables|Default|GetSM_Laurent)))))

(fn ConstructionScript)