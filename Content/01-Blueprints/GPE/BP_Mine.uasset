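; BP_Mine is a hazard that kills the diver when the player pawn touches it.
; On BeginPlay it caches the player pawn as BP_Diver.
; An overlap of its Sphere by that pawn plays a 2D explosion sound and controller force feedback, calls the diver's Death, then destroys the mine.
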(event OnComponentBeginOverlap(Sphere)
  (params (OverlappedComponent :type Primitive%20Component%20Object%20Reference) (OtherActor :type Actor%20Object%20Reference) (OtherComp :type Primitive%20Component%20Object%20Reference) (OtherBodyIndex :type Integer) (bFromSweep :type Boolean) (SweepResult :type Hit%20Result%20Structure%20%28by%20ref%29))
  (if (== OtherActor (Game|Player|GetPlayerPawn 0))
    (Audio|SpawnSound2D "/Game/07_SoundFX/Mine/MS_Explosion.MS_Explosion" 1.0 1.0 0.0 0)
    (Game|Feedback|ClientPlayForceFeedback (Game|GetPlayerController 0) "/Game/08_ForceFeedback/FF_Explosion.FF_Explosion" "None" false false false)
    (Default|Death (Variables|Default|GetAs%20BP%20Diver))
    (Actor|DestroyActor)))

(event EventBeginPlay
  (bind _asbp_diver (Utilities|Casting|CastToBP_Diver (Game|Player|GetPlayerPawn 0)))
  (Variables|Default|SetAs%20BP%20Diver _asbp_diver))

(fn ConstructionScript)