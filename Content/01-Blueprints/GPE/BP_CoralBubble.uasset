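; Coral bubble emitter that periodically releases bursts of BP_RefillBubble actors at its SpawnPoint.
; On BeginPlay it fires a burst immediately, then repeats it on a looping timer.
; Each burst runs through a local macro, a for-loop with a Delay between iterations, so the bubbles spawn staggered instead of all at once.
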(event Custom|SpawnBubble
  (Utilities|NewMacro 0 2 1.0
    (:then_0
      (Game|SpawnActorfromClass "/Game/01-Blueprints/GPE/BP_RefillBubble.BP_RefillBubble_C" (Math|Transform|MakeTransform (Transformation|GetSocketLocation (Variables|Default|GetSpawnPoint) "None") "0, 0, 0" "1.000000,1.000000,1.000000") "AlwaysSpawn" "MultiplyWithRoot" 0 0))))

(event EventBeginPlay
  (CallFunction|SpawnBubble)
  (Utilities|Time|SetTimerbyEvent (delegate Custom|SpawnBubble) 5.0 true))

(fn ConstructionScript)