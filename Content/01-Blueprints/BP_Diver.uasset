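; BP_Diver is a player-controlled diver with free 3D movement and controller-driven look, using Enhanced Input.
; Move input accelerates a Velocity vector along control-rotation axes and vertical input along world up, clamped to a max speed from a DataAsset.
; Tick applies Velocity through SetActorLocation without sweep, so movement ignores collision.
; On ticks without movement input, Velocity decays by a per-frame factor and debug prints show velocity and rotation.
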(event Input|EnhancedActionEvents|EnhancedInputActionIA_Move
  (params (ActionValue :type Vector%202D%20Structure) (ElapsedSeconds :type Float%20%28double-precision%29) (TriggeredSeconds :type Float%20%28double-precision%29) (InputAction :type Input%20Action%20Object%20Reference :default "/Game/01-Blueprints/Inputs/Actions/IA_Move.IA_Move"))
  (bind _returnvalue (Pawn|GetControlRotation :!class /Script/Engine.Pawn))
  (bind (_x _y) (Math|Vector2D|BreakVector2D ActionValue))
  (Variables|Default|SetVelocity (Math|Vector|ClampVectorSize (+ (* (Variables|/Game/01-Blueprints/BP_DA_Diver.BP_DA_Diver_C|GetAcceleration (Variables|Default|GetDataAsset)) (+ (* _x (Math|Vector|GetRightVector _returnvalue)) (* _y (Math|Vector|GetForwardVector _returnvalue)))) (Variables|Default|GetVelocity)) 0.0 (Variables|/Game/01-Blueprints/BP_DA_Diver.BP_DA_Diver_C|GetMaxVelocity (Variables|Default|GetDataAsset))))
  (Variables|Default|SetInputed true))

(event Input|EnhancedActionEvents|EnhancedInputActionIA_Look
  (params (ActionValue :type Vector%202D%20Structure) (ElapsedSeconds :type Float%20%28double-precision%29) (TriggeredSeconds :type Float%20%28double-precision%29) (InputAction :type Input%20Action%20Object%20Reference :default "/Game/01-Blueprints/Inputs/Actions/IA_Look.IA_Look"))
  (bind (_x _y) (Math|Vector2D|BreakVector2D ActionValue))
  (Pawn|Input|AddControllerYawInput _x)
  (Pawn|Input|AddControllerPitchInput _y))

(event Input|EnhancedActionEvents|EnhancedInputActionIA_Vertical
  (params (ActionValue :type Float%20%28double-precision%29) (ElapsedSeconds :type Float%20%28double-precision%29) (TriggeredSeconds :type Float%20%28double-precision%29) (InputAction :type Input%20Action%20Object%20Reference :default "/Game/01-Blueprints/Inputs/Actions/IA_Vertical.IA_Vertical"))
  (Variables|Default|SetVelocity (Math|Vector|ClampVectorSize (+ (* (Math|Vector|VectorUp) ActionValue (Variables|/Game/01-Blueprints/BP_DA_Diver.BP_DA_Diver_C|GetVerticalAcceleration (Variables|Default|GetDataAsset))) (Variables|Default|GetVelocity)) 0.0 (Variables|/Game/01-Blueprints/BP_DA_Diver.BP_DA_Diver_C|GetMaxVelocity (Variables|Default|GetDataAsset))))
  (Variables|Default|SetInputed true))

(event EventBeginPlay
  (Input|AddMappingContext (PlayerController|LocalPlayerSubsystems|GetEnhancedInputLocalPlayerSubsystem (Game|GetPlayerController 0)) "/Game/01-Blueprints/Inputs/IMC_Default.IMC_Default" 0 "(bIgnoreAllPressedKeysUntilRelease=True,bForceImmediately=False,bNotifyUserSettings=False)"))

(event EventTick
  (params (DeltaSeconds :type Float%20%28single-precision%29))
  (Transformation|SetActorLocation (+ (* DeltaSeconds (Variables|Default|GetVelocity)) (Transformation|GetActorLocation)) false false)
  (if (Variables|Default|GetInputed)
    (Variables|Default|SetInputed false)
    (else
      (bind _output_get (Variables|Default|SetVelocity (* (Variables|Default|GetVelocity) (Variables|/Game/01-Blueprints/BP_DA_Diver.BP_DA_Diver_C|GetVelocityDecay (Variables|Default|GetDataAsset)))))
      (Development|PrintString (Utilities|String|ToString(Vector) _output_get) true false "(R=0.973445,G=0.577580,B=0.016807,A=1.000000)" 0.0)
      (Development|PrintString (Utilities|String|ToString(Rotator) (Pawn|GetControlRotation :!class /Script/Engine.Pawn)) true false "(R=0.341914,G=0.445201,B=0.973445,A=1.000000)" 0.0))))

(fn ConstructionScript)