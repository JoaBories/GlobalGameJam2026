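; Player diver pawn that swims via Enhanced Input and FloatingPawnMovement, tuned by a data asset.
; Tick drains oxygen and any radiation countdown outside dialogue; either running low triggers fade, reset and respawn at PlayerStart.
; Sphere overlaps drive fish and shop prompts; pickup grabs wanted fish via GM_FIH, redeems completed sets or advances dialogue.
; Catching DA_RamFish stages a fake crash: throttled FPS, blue screen, quit; boost logic is disconnected.
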(event OnComponentBeginOverlap(Sphere)
  (params (OverlappedComponent :type Primitive%20Component%20Object%20Reference) (OtherActor :type Actor%20Object%20Reference) (OtherComp :type Primitive%20Component%20Object%20Reference) (OtherBodyIndex :type Integer) (bFromSweep :type Boolean) (SweepResult :type Hit%20Result%20Structure%20%28by%20ref%29))
  (Utilities|IsValid OtherActor
    (:Is%20Valid
      (if (Actor|ActorHasTag OtherActor "Fish")
        (bind _asbp_collectible_fish (Utilities|Casting|CastToBP_CollectibleFish OtherActor))
        (if (CallFunction|IsFishtoCatch _asbp_collectible_fish)
          (Default|ShowWidgetFish (Variables|/Game/01-Blueprints/GM_FIH.GM_FIH_C|GetHUD%20Chara (Variables|Default|GetAs%20GM%20FIH)))
          (Variables|Default|SetCurrentFish _asbp_collectible_fish))
        (elif (== OtherActor (Variables|Default|GetShop))
          (Default|Shop (Variables|/Game/01-Blueprints/GM_FIH.GM_FIH_C|GetHUD%20Chara (Variables|Default|GetAs%20GM%20FIH)) (Default|HasAllFishes (Variables|Default|GetAs%20GM%20FIH)) true))))))

(event OnComponentEndOverlap(Sphere)
  (params (OverlappedComponent :type Primitive%20Component%20Object%20Reference) (OtherActor :type Actor%20Object%20Reference) (OtherComp :type Primitive%20Component%20Object%20Reference) (OtherBodyIndex :type Integer))
  (if (Actor|ActorHasTag OtherActor "Fish")
    (if (== OtherActor (Variables|Default|GetCurrentFish))
      (Default|HideWidgetFish (Variables|/Game/01-Blueprints/GM_FIH.GM_FIH_C|GetHUD%20Chara (Variables|Default|GetAs%20GM%20FIH)))
      (Variables|Default|SetCurrentFish 0))
    (elif (== OtherActor (Variables|Default|GetShop))
      (Default|Shop (Variables|/Game/01-Blueprints/GM_FIH.GM_FIH_C|GetHUD%20Chara (Variables|Default|GetAs%20GM%20FIH)) false false))))

(event Custom|Death
  (bind _dataasset (Variables|Default|GetDataAsset))
  (Default|FadeBlackDie (Variables|Default|GetAs%20GM%20FIH))
  (Variables|Default|SetOxygen (Variables|/Game/01-Blueprints/Player/BP_DA_Diver.BP_DA_Diver_C|GetMaxOxygen _dataasset))
  (Variables|Default|SetTimer (Variables|/Game/01-Blueprints/Player/BP_DA_Diver.BP_DA_Diver_C|GetRadioactiveTimerLength _dataasset))
  (Variables|Default|SetisTimerOn false)
  (Default|CallOnUpdateRadioactive false 0.0)
  (Utilities|FlowControl|Delay 0.75)
  (bind _returnvalue (Actor|GetActorOfClass "/Script/Engine.PlayerStart"))
  (Transformation|SetActorLocation (Transformation|GetActorLocation _returnvalue) false false))

(event Custom|RefillOxygen
  (params (Amount :type Float%20%28double-precision%29))
  (bind _output_get (Variables|Default|SetOxygen (Math|Float|Clamp(Float) (+ Amount (Variables|Default|GetOxygen)) 0.0 (Variables|/Game/01-Blueprints/Player/BP_DA_Diver.BP_DA_Diver_C|GetMaxOxygen (Variables|Default|GetDataAsset)))))
  (Default|CallOnUpdateOxygen _output_get (Variables|/Game/01-Blueprints/Player/BP_DA_Diver.BP_DA_Diver_C|GetMaxOxygen (Variables|Default|GetDataAsset))))

(event Custom|StartTimerRadioactive
  (if (not (Variables|Default|GethaveRadioactiveMask))
    (Variables|Default|SetisTimerOn true)
    (Default|CallOnUpdateRadioactive true 1.0)))

(event Custom|BodSequence
  (Development|ExecuteConsoleCommand "t.MaxFPS 10" 0)
  (Utilities|FlowControl|Delay 5.0)
  (bind _returnvalue (UserInterface|CreateWidget "/Game/01-Blueprints/Uis/WBP_BlueScreen.WBP_BlueScreen_C"))
  (UserInterface|Viewport|AddtoViewport _returnvalue 15)
  (Utilities|FlowControl|Delay 5.0)
  (Game|QuitGame 0 "Quit" false))

(event Custom|StopTimer
  (Variables|Default|SetisTimerOn false)
  (Variables|Default|SetTimer (Variables|/Game/01-Blueprints/Player/BP_DA_Diver.BP_DA_Diver_C|GetRadioactiveTimerLength (Variables|Default|GetDataAsset)))
  (Default|CallOnUpdateRadioactive false 0.0))

(event Custom|ExitDialogue
  (Variables|/Script/Engine.MovementComponent|SetVelocity (Variables|Default|GetFloatingPawnMovement) "0, 0, 0")
  (Variables|Default|SetisInDialogue false))

(event Custom|GoInDialogue
  (Variables|/Script/Engine.MovementComponent|SetVelocity (Variables|Default|GetFloatingPawnMovement) "0, 0, 0")
  (Variables|Default|SetisInDialogue true))

(event Input|EnhancedActionEvents|EnhancedInputActionIA_Move
  (params (ActionValue :type Vector%202D%20Structure) (ElapsedSeconds :type Float%20%28double-precision%29) (TriggeredSeconds :type Float%20%28double-precision%29) (InputAction :type Input%20Action%20Object%20Reference :default "/Game/01-Blueprints/Inputs/Actions/IA_Move.IA_Move"))
  (bind _returnvalue (Pawn|GetControlRotation :!class /Script/Engine.Pawn))
  (bind (_x _y) (Math|Vector2D|BreakVector2D ActionValue))
  (bind _returnvalue_2 (Utilities|Time|GetWorldDeltaSeconds))
  (if (not (Variables|Default|GetisInDialogue))
    (Class|PawnMovementComponent|AddInputVector (Variables|Default|GetFloatingPawnMovement) (+ (* _x (Math|Vector|GetRightVector _returnvalue) _returnvalue_2 6e+01) (* _y (Math|Vector|GetForwardVector _returnvalue) _returnvalue_2 6e+01)) false)))

(event Input|EnhancedActionEvents|EnhancedInputActionIA_Look
  (params (ActionValue :type Vector%202D%20Structure) (ElapsedSeconds :type Float%20%28double-precision%29) (TriggeredSeconds :type Float%20%28double-precision%29) (InputAction :type Input%20Action%20Object%20Reference :default "/Game/01-Blueprints/Inputs/Actions/IA_Look.IA_Look"))
  (bind (_x _y) (Math|Vector2D|BreakVector2D ActionValue))
  (bind _returnvalue (Utilities|Time|GetWorldDeltaSeconds))
  (if (not (Variables|Default|GetisInDialogue))
    (Pawn|Input|AddControllerYawInput (* _x _returnvalue 6e+01))
    (Pawn|Input|AddControllerPitchInput (* _y _returnvalue 6e+01))))

(event Input|EnhancedActionEvents|EnhancedInputActionIA_Vertical
  (params (ActionValue :type Float%20%28double-precision%29) (ElapsedSeconds :type Float%20%28double-precision%29) (TriggeredSeconds :type Float%20%28double-precision%29) (InputAction :type Input%20Action%20Object%20Reference :default "/Game/01-Blueprints/Inputs/Actions/IA_Vertical.IA_Vertical"))
  (if (not (Variables|Default|GetisInDialogue))
    (Class|PawnMovementComponent|AddInputVector (Variables|Default|GetFloatingPawnMovement) (* ActionValue (Variables|/Game/01-Blueprints/Player/BP_DA_Diver.BP_DA_Diver_C|GetVerticalMult (Variables|Default|GetDataAsset)) (Math|Vector|VectorUp) (Utilities|Time|GetWorldDeltaSeconds) 6e+01) false)))

(event Input|EnhancedActionEvents|EnhancedInputActionIA_PickUpFish
  (params (ActionValue :type Boolean) (ElapsedSeconds :type Float%20%28double-precision%29) (TriggeredSeconds :type Float%20%28double-precision%29) (InputAction :type Input%20Action%20Object%20Reference :default "/Game/01-Blueprints/Inputs/Actions/IA_PickUpFish.IA_PickUpFish"))
  (if (not (Variables|Default|GetisInDialogue))
    (bind _currentfish (Variables|Default|GetCurrentFish)
      (:then
        (if (CallFunction|IsFishtoCatch _currentfish)
          (Default|SetGrabFish (Variables|Default|GetAs%20GM%20FIH) (Variables|/Game/01-Blueprints/GPE/Fishes/BP_CollectibleFish.BP_CollectibleFish_C|GetFish%20Data%20asset _currentfish))
          (if (== (Variables|/Game/01-Blueprints/GPE/Fishes/BP_CollectibleFish.BP_CollectibleFish_C|GetFish%20Data%20asset _currentfish) "/Game/01-Blueprints/GPE/Fishes/FishDataAssets/DA_RamFish.DA_RamFish")
            (CallFunction|BodSequence))
          (Default|DestroyFish _currentfish)))
      (:else
        (if (Utilities|Array|ContainsItem (Collision|GetOverlappingActors "/Game/01-Blueprints/GPE/BP_Shop.BP_Shop_C" :!class /Script/Engine.Actor) (Variables|Default|GetShop))
          (if (Default|HasAllFishes (Variables|Default|GetAs%20GM%20FIH))
            (Default|RedeemFish (Variables|Default|GetAs%20GM%20FIH))))))
    (else
      (Default|NextLine (Variables|Default|GetShop)))))

(event Input|EnhancedActionEvents|EnhancedInputActionIA_Boost
  (params (ActionValue :type Boolean) (ElapsedSeconds :type Float%20%28double-precision%29) (TriggeredSeconds :type Float%20%28double-precision%29) (InputAction :type Input%20Action%20Object%20Reference :default "/Game/01-Blueprints/Inputs/Actions/IA_Boost.IA_Boost"))
  ;[0.15 0.15 0.15 0.5] BoostAborted
)

(event Input|EnhancedActionEvents|EnhancedInputActionIA_Pause
  (params (ActionValue :type Boolean) (ElapsedSeconds :type Float%20%28double-precision%29) (TriggeredSeconds :type Float%20%28double-precision%29) (InputAction :type Input%20Action%20Object%20Reference :default "/Game/01-Blueprints/Inputs/Actions/IA_Pause.IA_Pause"))
  (Default|Pause (Variables|Default|GetAs%20GM%20FIH)))

(event EventBeginPlay
  (bind _dataasset (Variables|Default|GetDataAsset))
  (bind _asgm_fih (Utilities|Casting|CastToGM_FIH (Game|GetGameMode)))
  (Variables|Default|SetAs%20GM%20FIH _asgm_fih)
  (Input|AddMappingContext (PlayerController|LocalPlayerSubsystems|GetEnhancedInputLocalPlayerSubsystem (Game|GetPlayerController 0)) "/Game/01-Blueprints/Inputs/IMC_Default.IMC_Default" 0 "(bIgnoreAllPressedKeysUntilRelease=True,bForceImmediately=False,bNotifyUserSettings=False)")
  (Variables|Default|SetOxygen (Variables|/Game/01-Blueprints/Player/BP_DA_Diver.BP_DA_Diver_C|GetMaxOxygen _dataasset))
  (Variables|Default|SetTimer (Variables|/Game/01-Blueprints/Player/BP_DA_Diver.BP_DA_Diver_C|GetRadioactiveTimerLength _dataasset))
  (Default|CallOnUpdateRadioactive false 0.0)
  (Default|CallOnUpdateOxygen (Variables|Default|GetOxygen) (Variables|/Game/01-Blueprints/Player/BP_DA_Diver.BP_DA_Diver_C|GetMaxOxygen (Variables|Default|GetDataAsset)))
  (bind _returnvalue (Actor|GetActorOfClass "/Game/01-Blueprints/GPE/BP_Shop.BP_Shop_C"))
  (Variables|Default|SetShop _returnvalue))

(event EventTick
  (params (DeltaSeconds :type Float%20%28single-precision%29))
  (if (not (Variables|Default|GetisInDialogue))
    (CallFunction|UpdateOxygen DeltaSeconds)
    (if (Variables|Default|GetisTimerOn)
      (bind _output_get (Variables|Default|SetTimer (- (Variables|Default|GetTimer) DeltaSeconds)))
      (Development|PrintString (Utilities|String|ToString(Float) _output_get) true true "(R=0.000000,G=0.660000,B=1.000000,A=1.000000)" 0.0)
      (Default|CallOnUpdateRadioactive true (/ _output_get (Variables|/Game/01-Blueprints/Player/BP_DA_Diver.BP_DA_Diver_C|GetRadioactiveTimerLength (Variables|Default|GetDataAsset))))
      (if (<= (Variables|Default|GetTimer) 0.0)
        (CallFunction|Death)))))

(fn ConstructionScript
  (bind _dataasset (Variables|Default|GetDataAsset))
  (bind _floatingpawnmovement (Variables|Default|GetFloatingPawnMovement))
  (Variables|/Script/Engine.FloatingPawnMovement|SetAcceleration _floatingpawnmovement (Variables|/Game/01-Blueprints/Player/BP_DA_Diver.BP_DA_Diver_C|GetAcceleration _dataasset))
  (Variables|/Script/Engine.FloatingPawnMovement|SetMaxSpeed _floatingpawnmovement (Variables|/Game/01-Blueprints/Player/BP_DA_Diver.BP_DA_Diver_C|GetMaxSpeed _dataasset))
  (Variables|/Script/Engine.FloatingPawnMovement|SetDeceleration _floatingpawnmovement (Variables|/Game/01-Blueprints/Player/BP_DA_Diver.BP_DA_Diver_C|GetDecceleration _dataasset))
  (Variables|/Script/Engine.FloatingPawnMovement|SetTurningBoost _floatingpawnmovement (Variables|/Game/01-Blueprints/Player/BP_DA_Diver.BP_DA_Diver_C|GetTurningBoost _dataasset))
  (Components|Sphere|SetSphereRadius (Variables|Default|GetSphere) (Variables|/Game/01-Blueprints/Player/BP_DA_Diver.BP_DA_Diver_C|GetSphereRadius (Variables|Default|GetDataAsset)) true))

(fn UpdateOxygen
  (params (Delta :type Float%20%28double-precision%29))
  (bind _output_get (Variables|Default|SetOxygen (- (Variables|Default|GetOxygen) (* Delta (Variables|/Game/01-Blueprints/Player/BP_DA_Diver.BP_DA_Diver_C|GetOxygenDecay (Variables|Default|GetDataAsset))))))
  (Default|CallOnUpdateOxygen _output_get (Variables|/Game/01-Blueprints/Player/BP_DA_Diver.BP_DA_Diver_C|GetMaxOxygen (Variables|Default|GetDataAsset)))
  (if (<= (Variables|Default|GetOxygen) (Variables|/Game/01-Blueprints/Player/BP_DA_Diver.BP_DA_Diver_C|GetLowOxygen (Variables|Default|GetDataAsset)))
    (CallFunction|Death)
    (else
      (Development|PrintString (Utilities|String|ToString(Float) (Variables|Default|GetOxygen)) true false "(R=0.039546,G=0.651406,B=0.000000,A=1.000000)" 0.0))))

(fn IsFishtoCatch
  (params (Fish :type BP%20Collectible%20Fish%20Object%20Reference))
  (return (Utilities|Map|Contains (Variables|/Game/01-Blueprints/GM_FIH.GM_FIH_C|GetFishToCatch (Variables|Default|GetAs%20GM%20FIH)) (Variables|/Game/01-Blueprints/GPE/Fishes/BP_CollectibleFish.BP_CollectibleFish_C|GetFish%20Data%20asset Fish))))