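; YELO submarine environment Blueprint that animates nine cylinder components, treated as plates, with a continuous sway and bob.
; StartMove, called from BeginPlay and the construction script, gives each plate a random phase offset and starts a looping timer.
; MovePlates advances a time counter and adds sine-based relative location deltas: a shared diagonal XY sway plus an individually phased Z bob.
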(event Custom|move%20plates
  (Variables|Default|Settime (+ (Variables|Default|Gettime) 0.05))
  (for (_array_element _array_index) (Utilities|Array|MakeArray (Variables|Default|GetCylinder_035) (Variables|Default|GetCylinder_032) (Variables|Default|GetCylinder_036) (Variables|Default|GetCylinder_037) (Variables|Default|GetCylinder_031) (Variables|Default|GetCylinder_030) (Variables|Default|GetCylinder_023) (Variables|Default|GetCylinder_033) (Variables|Default|GetCylinder_034))
    (Transformation|AddRelativeLocation _array_element (Math|Vector|MakeVector (* (+ (Math|Trig|Sin(Degrees) (* (Variables|Default|Gettime) 7.0)) 0.0) 0.3) (* (+ (Math|Trig|Sin(Degrees) (* (Variables|Default|Gettime) 7.0)) 0.0) 0.3) (* (Math|Trig|Sin(Degrees) (* (+ (Utilities|Array|Get(acopy) (Variables|Default|Gettime%20delay) _array_index) (Variables|Default|Gettime)) 1e+01)) 0.12)) false false)))

(event Custom|start%20Move
  (for _array_element (Utilities|Array|MakeArray (Variables|Default|GetCylinder_035) (Variables|Default|GetCylinder_032) (Variables|Default|GetCylinder_036) (Variables|Default|GetCylinder_037) (Variables|Default|GetCylinder_031) (Variables|Default|GetCylinder_030) (Variables|Default|GetCylinder_023) (Variables|Default|GetCylinder_033) (Variables|Default|GetCylinder_034))
    (Utilities|Array|Add (Variables|Default|Gettime%20delay) (Math|Random|RandomFloatinRange 0.0 3.6e+02)))
  (Variables|Default|Settime 1.8e+02)
  (Utilities|Time|SetTimerbyEvent (delegate Custom|move%20plates) 0.05 true))

(event EventBeginPlay
  (CallFunction|StartMove))

(fn ConstructionScript
  (CallFunction|StartMove))